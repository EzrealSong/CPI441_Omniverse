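; GlassDivider is an interactable machine that opens a GlassDividerUI widget and sets the thickness of bottles inside its box.
; The box shows a text prompt while the first-person character overlaps it.
; Looping timers from BeginPlay forward MoveArrow to the widget and drain Health while its power button is on.
; Setthickness assigns each overlapping BP_TestBottles a thickness from the HighPressure and LowPressure flags.
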(event OnComponentBeginOverlap(Box)
  (params (OverlappedComponent :type Primitive%20Component%20Object%20Reference) (OtherActor :type Actor%20Object%20Reference) (OtherComp :type Primitive%20Component%20Object%20Reference) (OtherBodyIndex :type Integer) (bFromSweep :type Boolean) (SweepResult :type Hit%20Result%20Structure%20%28by%20ref%29))
  (Utilities|Casting|CastToBP_FirstPersonCharacter OtherActor)
  (Development|SetHiddeninGame (Variables|Default|GetTextRender) false false))

(event OnComponentEndOverlap(Box)
  (params (OverlappedComponent :type Primitive%20Component%20Object%20Reference) (OtherActor :type Actor%20Object%20Reference) (OtherComp :type Primitive%20Component%20Object%20Reference) (OtherBodyIndex :type Integer))
  (Utilities|Casting|CastToBP_FirstPersonCharacter OtherActor)
  (Development|SetHiddeninGame (Variables|Default|GetTextRender) true false))

(event Custom|Lose%20Health
  (bind _asglass_divider_ui (Utilities|Casting|CastToGlassDividerUI (Variables|Default|GetGlassDividerUIRef)))
  (if (Variables|/Game/UIElements/GlassDividerUI.GlassDividerUI_C|GetPowerButtonOnBool _asglass_divider_ui)
    (Variables|Default|Sethealth (Math|Float|Clamp(Float) (- (Variables|Default|Gethealth) 5.0) 0.0 1e+02))))

(event Custom|MoveArrow
  (bind _asglass_divider_ui (Utilities|Casting|CastToGlassDividerUI (Variables|Default|GetGlassDividerUIRef)))
  (Default|MoveArrow _asglass_divider_ui))

(event Custom|Set%20thickness
  (for _array_element (Collision|GetOverlappingActors (Variables|Default|GetBox) "/Game/Blueprints/BP_TestBottles.BP_TestBottles_C" :!class /Script/Engine.PrimitiveComponent)
    (bind _asbp_test_bottles (Utilities|Casting|CastToBP_TestBottles _array_element))
    (if (Variables|Default|Gethigh%20pressure)
      (Variables|/Game/Blueprints/BP_TestBottles.BP_TestBottles_C|SetThickness _asbp_test_bottles 2)
      (elif (Variables|Default|Getlow%20pressure)
        (Variables|/Game/Blueprints/BP_TestBottles.BP_TestBottles_C|SetThickness _asbp_test_bottles 1)
        (else
          (Variables|/Game/Blueprints/BP_TestBottles.BP_TestBottles_C|SetThickness _asbp_test_bottles 3))))))

(event Collision|EventActorBeginOverlap
  (params (OtherActor :type Actor%20Object%20Reference)))

(event EventTick
  (params (DeltaSeconds :type Float%20%28single-precision%29)))

(event EventInteract
  (bind _returnvalue (UserInterface|CreateWidget "/Game/UIElements/GlassDividerUI.GlassDividerUI_C"))
  (bind _output_get (Variables|Default|SetGlassDividerUIRef _returnvalue))
  (UserInterface|Viewport|AddtoViewport _output_get 0))

(event EventBeginPlay
  (CallFunction|StartTimer))

(fn ConstructionScript)

(fn StartTimer
  (Utilities|Time|SetTimerbyFunctionName 0 "Lose Health" 1.0 true)
  (Utilities|Time|SetTimerbyFunctionName 0 "MoveArrow" 0.1 true))

(fn Startimerupdatehealth)