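; BottlePricer is an actor that turns bottles placed inside its box into score for the player.
; Every tick it polls the box for overlapping BP_TestBottles and prices each as the product of thickness, clarity and brittleness, scaled down by a constant.
; It prints that price, passes it to UpdateScore on the first-person character's PlayerUI, then destroys the bottle.
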(event EventTick
  (params (DeltaSeconds :type Float%20%28single-precision%29))
  (for _array_element (Collision|GetOverlappingActors (Variables|Default|GetBox) "/Game/Blueprints/BP_TestBottles.BP_TestBottles_C" :!class /Script/Engine.PrimitiveComponent)
    (bind _asbp_test_bottles (Utilities|Casting|CastToBP_TestBottles _array_element))
    (bind _returnvalue (Actor|GetActorOfClass "/Game/FirstPerson/Blueprints/BP_FirstPersonCharacter.BP_FirstPersonCharacter_C"))
    (bind _asbp_first_person_character (Utilities|Casting|CastToBP_FirstPersonCharacter _returnvalue))
    (Development|PrintString (Utilities|String|ToString(Float) (Math|Conversions|ToFloat(Integer) (/ (Math|Conversions|ToFloat(Integer) (* (* (Variables|/Game/Blueprints/BP_TestBottles.BP_TestBottles_C|GetThickness _asbp_test_bottles) (Variables|/Game/Blueprints/BP_TestBottles.BP_TestBottles_C|GetClarity _asbp_test_bottles)) (Variables|/Game/Blueprints/BP_TestBottles.BP_TestBottles_C|GetBrittleness _asbp_test_bottles))) 12.0))))
    (Default|UpdateScore (Variables|/Game/FirstPerson/Blueprints/BP_FirstPersonCharacter.BP_FirstPersonCharacter_C|GetPlayerUI _asbp_first_person_character) (Math|Conversions|ToFloat(Integer) (/ (Math|Conversions|ToFloat(Integer) (* (* (Variables|/Game/Blueprints/BP_TestBottles.BP_TestBottles_C|GetThickness _asbp_test_bottles) (Variables|/Game/Blueprints/BP_TestBottles.BP_TestBottles_C|GetClarity _asbp_test_bottles)) (Variables|/Game/Blueprints/BP_TestBottles.BP_TestBottles_C|GetBrittleness _asbp_test_bottles))) 12.0)))
    (Actor|DestroyActor _array_element)))

(fn ConstructionScript)