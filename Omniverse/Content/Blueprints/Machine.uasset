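; Production machine that turns InputMaterial actors entering its box into spawned test bottles, with an interactable MachineUi widget.
; Overlapping material is destroyed to add capacity until full, and each bottle consumes capacity.
; Looping timers from StartTimer lower health and raise temperature while the UI power button is on.
; Temperature bands set the bottle spawn Delay, shorter when hotter, though spawning itself ignores power state.
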(event OnComponentBeginOverlap(Box)
  (params (OverlappedComponent :type Primitive%20Component%20Object%20Reference) (OtherActor :type Actor%20Object%20Reference) (OtherComp :type Primitive%20Component%20Object%20Reference) (OtherBodyIndex :type Integer) (bFromSweep :type Boolean) (SweepResult :type Hit%20Result%20Structure%20%28by%20ref%29))
  (bind _output_get (Variables|Default|SetCapacity (>= (Variables|Default|Getcurrentcapacity) (Variables|Default|Getmaxcapacity))))
  (if (not _output_get)
    (Utilities|Casting|CastToInputMaterial OtherActor)
    (Variables|Default|Setcurrentcapacity (+ (Variables|Default|Getcurrentcapacity) 10))
    (Actor|DestroyActor OtherActor)))

(event Custom|Lose%20Health
  (bind _asmachine_ui (Utilities|Casting|CastToMachineUi (Variables|Default|GetMachineUIref)))
  (if (Variables|/Game/UI/UI_Blueprints/MachineUi.MachineUi_C|GetPowerButtonOnBool _asmachine_ui)
    (Variables|Default|Sethealth (Math|Float|Clamp(Float) (- (Variables|Default|Gethealth) 5.0) 0.0 1e+02))
    (if (<= (Variables|Default|Gethealth) 0.0)
      (Variables|Default|Settemperaturecheck true)
      (else
        (Variables|Default|Settemperaturecheck false)))))

(event Custom|Bottle%20Speed
  (if (Variables|Default|Gettemp%20low)
    (Variables|Default|Settimer 1e+01)
    (elif (Variables|Default|Gettemp%20med)
      (Variables|Default|Settimer 5.0)
      (elif (Variables|Default|Gettemp%20high)
        (Variables|Default|Settimer 1.0)
        (else
          (Variables|Default|Settimer 0.0))))))

(event Custom|Set%20Temp%20Range
  (Variables|Default|Settemp%20low (Math|Float|InRange(Float) (Variables|Default|GetTemperature) 3.5e+02 483.0))
  (Variables|Default|Settemp%20med (Math|Float|InRange(Float) (Variables|Default|GetTemperature) 484.0 616.0))
  (Variables|Default|Settemp%20high (Math|Float|InRange(Float) (Variables|Default|GetTemperature) 617.0 7.5e+02))
  (CallFunction|BottleSpeed))

(event Custom|GainTemp
  (CallFunction|SetTempRange)
  (CallFunction|CustomEvent)
  (bind _asmachine_ui (Utilities|Casting|CastToMachineUi (Variables|Default|GetMachineUIref)))
  (if (Variables|/Game/UI/UI_Blueprints/MachineUi.MachineUi_C|GetPowerButtonOnBool _asmachine_ui)
    (if (> (Variables|Default|GetMaxTemp) (Variables|Default|GetTemperature))
      (Variables|Default|SetTemperature (Math|Float|Clamp(Float) (+ (Variables|Default|GetTemperature) 1.0) 0.0 7.5e+02))
      (Variables|Default|Settemperaturecheck false)
      (else
        (Variables|Default|Settemperaturecheck true)))))

(event Custom|Start
  (bind _returnvalue (UserInterface|CreateWidget "/Game/UI/UI_Blueprints/MachineUi.MachineUi_C"))
  (Variables|Default|SetMachineUIref _returnvalue)
  (CallFunction|StartTimer)
  (Variables|Default|Settest 10))

(event Custom|CustomEvent
  (if (not (== (Variables|Default|Getcurrentcapacity) 0))
    (Utilities|FlowControl|Delay (Variables|Default|Gettimer))
    (Game|SpawnActorfromClass "/Game/Blueprints/BP_TestBottles.BP_TestBottles_C" (Math|Conversions|ToTransform(Vector) (+ (Transformation|GetWorldLocation (Variables|Default|GetCube)) "400.000000,0.000000,-150.000000")) "Undefined" 0 0)
    (Variables|Default|Setcurrentcapacity (- (Variables|Default|Getcurrentcapacity) 10))))

(event Collision|EventActorBeginOverlap
  (params (OtherActor :type Actor%20Object%20Reference)))

(event EventInteract
  (bind _returnvalue (UserInterface|CreateWidget "/Game/UI/UI_Blueprints/MachineUi.MachineUi_C"))
  (bind _output_get (Variables|Default|SetMachineUIref _returnvalue))
  (UserInterface|Viewport|AddtoViewport _output_get 0))

(fn ConstructionScript)

(fn StartTimer
  (Utilities|Time|SetTimerbyFunctionName 0 "Lose Health" 1.0 true)
  (Utilities|Time|SetTimerbyFunctionName 0 "GainTemp" 1.0 true))

(fn Startimerupdatehealth)