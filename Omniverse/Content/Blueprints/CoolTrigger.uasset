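; Trigger actor that applies a selectable brittleness level to test bottles inside its box.
; Every Tick it polls overlapping BP_TestBottles, writes the current level to their Brittleness, sets their Progress and refreshes their glass appearance.
; Tick also polls number keys on the first player controller to switch between three levels, recoloring the cube red, green or blue to match.
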(event EventBeginPlay
  (Variables|Default|SetVariable 1))

(event EventTick
  (params (DeltaSeconds :type Float%20%28single-precision%29))
  (for _array_element (Collision|GetOverlappingActors (Variables|Default|GetBox) "/Game/Blueprints/BP_TestBottles.BP_TestBottles_C" :!class /Script/Engine.PrimitiveComponent)
    (bind _asbp_test_bottles (Utilities|Casting|CastToBP_TestBottles _array_element))
    (Variables|/Game/Blueprints/BP_TestBottles.BP_TestBottles_C|SetBrittleness _asbp_test_bottles (Variables|Default|GetVariable))
    (Variables|/Game/Blueprints/BP_TestBottles.BP_TestBottles_C|SetProgress _asbp_test_bottles 1)
    (Default|ChangeGlassAppearance _asbp_test_bottles))
  (if (Game|Player|IsInputKeyDown (Game|GetPlayerController 0) "Four")
    (Variables|Default|SetVariable 1)
    (Rendering|Material|SetMaterial (Variables|Default|GetCube) 0 "/Game/Materials/CustomMaterial/M_BasicRed.M_BasicRed")
    (elif (Game|Player|IsInputKeyDown (Game|GetPlayerController 0) "Five")
      (Variables|Default|SetVariable 2)
      (Rendering|Material|SetMaterial (Variables|Default|GetCube) 0 "/Game/Materials/CustomMaterial/M_BasicGreen.M_BasicGreen")
      (elif (Game|Player|IsInputKeyDown (Game|GetPlayerController 0) "Six")
        (Variables|Default|SetVariable 3)
        (Rendering|Material|SetMaterial (Variables|Default|GetCube) 0 "/Game/Materials/CustomMaterial/M_BasicBlue.M_BasicBlue")))))

(fn ConstructionScript)