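; BP_ConveyorBelt is a conveyor belt actor that carries test bottles along its surface.
; Each Tick it gathers actors overlapping the Conveyor component and casts them to BP_TestBottles.
; Matching bottles are moved by an unswept world offset along the Arrow component's forward vector, scaled by Speed and delta time, so the arrow sets the belt direction.
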(event EventTick
  (params (DeltaSeconds :type Float%20%28single-precision%29))
  (for _array_element (Collision|GetOverlappingActors (Variables|Default|GetConveyor) 0 :!class /Script/Engine.PrimitiveComponent)
    (bind _asbp_test_bottles (Utilities|Casting|CastToBP_TestBottles _array_element))
    (Transformation|AddActorWorldOffset _asbp_test_bottles (* (* DeltaSeconds (Variables|Default|Getspeed)) (Math|Vector|GetForwardVector (Transformation|GetWorldRotation (Variables|Default|GetArrow)))))))

(fn ConstructionScript)