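; Cooler machine actor that spends coolant to set the Clarity of overlapping test bottles and update their glass appearance.
; Each overlap drains the capacity; once empty, bottles get zero Clarity.
; Interact opens the main UI, and Tick refills coolant while RefillingBool is set, updating main and repair UIs.
; BeginPlay loops a timer on "Set thickness", absent here; box-scan and health-decay logic never run.
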(event Collision|EventActorBeginOverlap
  (params (OtherActor :type Actor%20Object%20Reference))
  (if (> (Variables|Default|GetCurrentCapacity) 0.0)
    (bind _asbp_test_bottles (Utilities|Casting|CastToBP_TestBottles OtherActor))
    (Variables|/Game/Blueprints/BP_TestBottles.BP_TestBottles_C|SetClarity _asbp_test_bottles (Variables|Default|GetOpacity))
    (Default|ChangeGlassAppearance _asbp_test_bottles)
    (if (< (- (Variables|Default|GetCurrentCapacity) 5.0) 0.0)
      (bind _output_get (Variables|Default|SetCurrentCapacity 0.0))
      (else
        (Variables|Default|SetCurrentCapacity (- (Variables|Default|GetCurrentCapacity) 5.0))))
    (Default|UpdateCoolant (Variables|Default|GetCoolerMainUIRef) _output_get)
    (if (Variables|Default|GetRepairCreated)
      (Default|UpdateBar (Variables|Default|GetCoolerRepairUIRef)))
    (else
      (bind _asbp_test_bottles_2 (Utilities|Casting|CastToBP_TestBottles OtherActor))
      (Variables|/Game/Blueprints/BP_TestBottles.BP_TestBottles_C|SetClarity _asbp_test_bottles_2 0))))

(event EventTick
  (params (DeltaSeconds :type Float%20%28single-precision%29))
  (if (< (Variables|Default|GetCurrentCapacity) (Variables|Default|GetMaxCapacity))
    (if (Variables|Default|GetRefillingBool)
      (bind _output_get (Variables|Default|SetCurrentCapacity (+ (Variables|Default|GetCurrentCapacity) 0.5)))
      (Default|UpdateCoolant (Variables|Default|GetCoolerMainUIRef) _output_get)
      (Default|UpdateBar (Variables|Default|GetCoolerRepairUIRef)))))

(event EventInteract
  (bind _returnvalue (UserInterface|CreateWidget "/Game/UI/UI_Blueprints/CoolerMainUI.CoolerMainUI_C"))
  (bind _output_get (Variables|Default|SetCoolerMainUIRef _returnvalue))
  (UserInterface|Viewport|AddtoViewport _output_get 0)
  (Default|UpdateCoolant (Variables|Default|GetCoolerMainUIRef) (Variables|Default|GetCurrentCapacity)))

(event EventBeginPlay
  (CallFunction|StartTimer)
  (Variables|Default|SetOpacity 1)
  (bind _output_get (Variables|Default|SetMaxCapacity 1e+02))
  (Variables|Default|SetCurrentCapacity _output_get))

(fn ConstructionScript)

(fn StartTimer
  (Utilities|Time|SetTimerbyFunctionName 0 "Set thickness" 1.0 true))

(fn Startimerupdatehealth)