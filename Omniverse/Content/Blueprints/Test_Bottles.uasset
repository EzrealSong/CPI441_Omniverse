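; Test Blueprint that swaps the look of a bottle component while a key is held.
; BeginPlay sets the glass property variables (progress, thickness, brittleness, clarity) to an unset-style negative value, and nothing here reads them.
; Tick polls the first player controller for the key and calls ChangeGlassAppearance, which sets the first material slot of ASUBottle to M_BaseMetal, with no revert.
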(event Custom|Change%20Glass%20Appearance
  (Rendering|Material|SetMaterial (Variables|Default|GetASU_bottle) 0 "/Game/Materials/M_BaseMetal.M_BaseMetal"))

(event EventBeginPlay
  (Variables|Default|SetProgress -1)
  (Variables|Default|SetThickness -1)
  (Variables|Default|SetBrittleness -1)
  (Variables|Default|SetClarity -1))

(event EventTick
  (params (DeltaSeconds :type Float%20%28single-precision%29))
  (if (Game|Player|IsInputKeyDown (Game|GetPlayerController 0) "One")
    (CallFunction|ChangeGlassAppearance)))

(fn ConstructionScript)