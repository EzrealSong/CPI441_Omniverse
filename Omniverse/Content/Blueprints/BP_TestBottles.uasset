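; BP_TestBottles is a test glass bottle Blueprint that shows stages of glass cooling through material swaps.
; The ChangeGlassAppearance event maps Progress to a molten, semi-cooled or new glass material on the ASUBottle component.
; BeginPlay initializes the glass properties and calls that event, so the bottle starts semi-cooled.
; Thickness, Brittleness and Clarity are set but do not affect the appearance here.
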(event Custom|Change%20Glass%20Appearance
  (if (== 0 (Variables|Default|GetProgress))
    (Rendering|Material|SetMaterial (Variables|Default|GetASU_bottle) 0 "/Game/Materials/CustomMaterial/M_MoltenGlass.M_MoltenGlass")
    (elif (== 1 (Variables|Default|GetProgress))
      (Rendering|Material|SetMaterial (Variables|Default|GetASU_bottle) 0 "/Game/Materials/CustomMaterial/M_SemiCooled_Glass.M_SemiCooled_Glass")
      (elif (== 2 (Variables|Default|GetProgress))
        (Rendering|Material|SetMaterial (Variables|Default|GetASU_bottle) 0 "/Game/Materials/CustomMaterial/M_NewGlass.M_NewGlass")))))

(event EventBeginPlay
  (Variables|Default|SetProgress 1)
  (Variables|Default|SetThickness 1)
  (Variables|Default|SetBrittleness 1)
  (Variables|Default|SetClarity 1)
  (CallFunction|ChangeGlassAppearance))

(fn ConstructionScript)