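; Pressure station actor that sets the brittleness of test bottles from a pressure gauge and opens a PressureStationUi widget on Interact.
; Looping timers started at BeginPlay drain Health and lower the gauge arrow angle, which Tick maps to three pressure levels.
; Overlapping bottles get brittleness from that angle and update their glass appearance, or get zero brittleness when Health is depleted.
; The Box destroys InputMaterial actors entering it.
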(event OnComponentBeginOverlap(Box)
  (params (OverlappedComponent :type Primitive%20Component%20Object%20Reference) (OtherActor :type Actor%20Object%20Reference) (OtherComp :type Primitive%20Component%20Object%20Reference) (OtherBodyIndex :type Integer) (bFromSweep :type Boolean) (SweepResult :type Hit%20Result%20Structure%20%28by%20ref%29))
  (if true
    (Utilities|Casting|CastToInputMaterial OtherActor)
    (Actor|DestroyActor OtherActor)))

(event Custom|LoseHealth
  (Variables|Default|Sethealth (Math|Float|Clamp(Float) (- (Variables|Default|Gethealth) 5.0) 0.0 1e+02)))

(event Custom|LosePressure
  (if (not (Variables|Default|GetIsAngleArrowNeg90))
    (Variables|Default|SetAngleofArrow (- (Variables|Default|GetAngleofArrow) 0.2))))

(event Custom|Lose%20Health
  (if (> (Variables|Default|Gethealth) 0.0)
    (Variables|Default|Sethealth (Math|Float|Clamp(Float) (- (Variables|Default|Gethealth) 1.0) 0.0 1e+02))))

(event Custom|Set%20Brittleness)

(event Collision|EventActorBeginOverlap
  (params (OtherActor :type Actor%20Object%20Reference))
  (if (> (Variables|Default|Gethealth) 0.0)
    (bind _asbp_test_bottles (Utilities|Casting|CastToBP_TestBottles OtherActor))
    (if (>= (Variables|Default|GetAngleofArrow) 43)
      (Variables|/Game/Blueprints/BP_TestBottles.BP_TestBottles_C|SetBrittleness _asbp_test_bottles 3)
      (elif (>= (Variables|Default|GetAngleofArrow) -38)
        (Variables|/Game/Blueprints/BP_TestBottles.BP_TestBottles_C|SetBrittleness _asbp_test_bottles 2)
        (else
          (Variables|/Game/Blueprints/BP_TestBottles.BP_TestBottles_C|SetBrittleness _asbp_test_bottles 1))))
    (Default|ChangeGlassAppearance _asbp_test_bottles)
    (else
      (bind _asbp_test_bottles_2 (Utilities|Casting|CastToBP_TestBottles OtherActor))
      (Variables|/Game/Blueprints/BP_TestBottles.BP_TestBottles_C|SetBrittleness _asbp_test_bottles_2 0))))

(event EventTick
  (params (DeltaSeconds :type Float%20%28single-precision%29))
  (if (>= (Variables|Default|GetAngleofArrow) 43.0)
    (Variables|Default|SetPressure 2)
    (elif (>= (Variables|Default|GetAngleofArrow) -38.0)
      (Variables|Default|SetPressure 1)
      (else
        (Variables|Default|SetPressure 0))))
  (if (<= (Variables|Default|GetAngleofArrow) -90)
    (Variables|Default|SetIsAngleArrowNeg90 true)
    (else
      (Variables|Default|SetIsAngleArrowNeg90 false))))

(event EventInteract
  (bind _returnvalue (UserInterface|CreateWidget "/Game/UI/UI_Blueprints/PressureStationUi.PressureStationUi_C"))
  (bind _output_get (Variables|Default|SetPressureUIRef _returnvalue))
  (UserInterface|Viewport|AddtoViewport _output_get 0))

(event EventBeginPlay
  (CallFunction|StartTimer))

(fn ConstructionScript)

(fn StartTimer
  (Utilities|Time|SetTimerbyFunctionName 0 "Lose Health" 1.0 true)
  (Utilities|Time|SetTimerbyFunctionName 0 "LosePressure" 0.2 true))

(fn Startimerupdatehealth)