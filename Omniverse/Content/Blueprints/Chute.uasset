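; Interactable chute actor that spawns InputMaterial actors, loses health over time and feeds sand, lime and soda values to its BP_Chute widget.
; A box overlap toggles the text prompt for the first-person character, and Interact adds the widget to the viewport.
; A looping timer drains health, while a Delay on Tick throttles spawning at an offset from the cube until StopSpawn is set.
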(event OnComponentBeginOverlap(Box)
  (params (OverlappedComponent :type Primitive%20Component%20Object%20Reference) (OtherActor :type Actor%20Object%20Reference) (OtherComp :type Primitive%20Component%20Object%20Reference) (OtherBodyIndex :type Integer) (bFromSweep :type Boolean) (SweepResult :type Hit%20Result%20Structure%20%28by%20ref%29))
  (Utilities|Casting|CastToBP_FirstPersonCharacter OtherActor)
  (Development|SetHiddeninGame (Variables|Default|GetTextRender) false false))

(event OnComponentEndOverlap(Box)
  (params (OverlappedComponent :type Primitive%20Component%20Object%20Reference) (OtherActor :type Actor%20Object%20Reference) (OtherComp :type Primitive%20Component%20Object%20Reference) (OtherBodyIndex :type Integer))
  (Utilities|Casting|CastToBP_FirstPersonCharacter OtherActor)
  (Development|SetHiddeninGame (Variables|Default|GetTextRender) true false))

(event Custom|Lose%20Health
  (Variables|Default|Sethealth (Math|Float|Clamp(Float) (- (Variables|Default|Gethealth) 0.25) 0.0 1e+02)))

(event Custom|SetLime
  (Variables|/Game/UI/UI_Blueprints/BP_Chute.BP_Chute_C|SetLime_Float (Variables|Default|GetChuteRef) (Variables|Default|GetLime_F)))

(event Custom|SetSand
  (Variables|/Game/UI/UI_Blueprints/BP_Chute.BP_Chute_C|SetSand_Float (Variables|Default|GetChuteRef) (Variables|Default|GetSand_F)))

(event Custom|SetSoda
  (Variables|/Game/UI/UI_Blueprints/BP_Chute.BP_Chute_C|SetSoda_Float (Variables|Default|GetChuteRef) (Variables|Default|GetSoda_F)))

(event Collision|EventActorBeginOverlap
  (params (OtherActor :type Actor%20Object%20Reference)))

(event EventTick
  (params (DeltaSeconds :type Float%20%28single-precision%29))
  (if (not (Variables|Default|GetStopSpawn))
    (Utilities|FlowControl|Delay 3.0)
    (Game|SpawnActorfromClass "/Game/Blueprints/InputMaterial.InputMaterial_C" (Math|Conversions|ToTransform(Vector) (+ (Transformation|GetWorldLocation (Variables|Default|GetCube)) "0.000000,660.000000,200.000000")) "Undefined" 0 0)))

(event EventInteract
  (UserInterface|Viewport|AddtoViewport (Variables|Default|GetChuteRef) 0))

(event EventBeginPlay
  (CallFunction|StartTimer)
  (bind _returnvalue (UserInterface|CreateWidget "/Game/UI/UI_Blueprints/BP_Chute.BP_Chute_C"))
  (bind _output_get (Variables|Default|SetChuteRef _returnvalue))
  (Default|StartTimer _output_get))

(fn ConstructionScript)

(fn StartTimer
  (Utilities|Time|SetTimerbyFunctionName 0 "Lose Health" 1.0 true))

(fn Startimerupdatehealth)